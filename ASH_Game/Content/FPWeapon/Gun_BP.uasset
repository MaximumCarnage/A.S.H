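; Weapon actor for the TopDownCharacter that manages an aim indicator and gun mesh shadows as the player switches to first person.
; Tick polls the character's death and view state, triggering a one-time delayed reveal of Aim and shadow disabling, or reverting them outside first person.
; Left click only flags the character Empty when Bulletcount is zero or below.
; The bullet, effect, sound and ammo-decrement firing chain is disconnected and never runs.
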(event Custom|Activate_FirstPerson
  (Utilities|FlowControl|Delay 6.0)
  (Rendering|SetVisibility (Variables|Default|GetAim) true false)
  (Utilities|FlowControl|Delay 2.0)
  (Rendering|SetCastShadow (Variables|Default|GetACWR_MAG) false))

(event EventBeginPlay
  (Rendering|SetVisibility (Variables|Default|GetAim) false false))

(event Collision|EventActorBeginOverlap
  (params (OtherActor :type Actor%20Object%20Reference)))

(event EventTick
  (params (DeltaSeconds :type Float%20%28single-precision%29))
  (bind _astop_down_character (Utilities|Casting|CastToTopDownCharacter (Game|GetPlayerCharacter 0)))
  (if (Variables|/Game/TopDownBP/Blueprints/TopDownCharacter.TopDownCharacter_C|GetCharacter_Is_Death _astop_down_character)
    (Rendering|SetVisibility (Variables|Default|GetArrow) false false)
    (elif (Variables|/Game/TopDownBP/Blueprints/TopDownCharacter.TopDownCharacter_C|GetSwitch_To_First_Person _astop_down_character)
      (Utilities|FlowControl|Sequence
        (:then_0
          (Utilities|FlowControl|DoOnce false
            (:Completed
              (CallFunction|ActivateFirstPerson)))))
      (else
        (Rendering|SetVisibility (Variables|Default|GetAim) false false)
        (Rendering|SetCastShadow (Variables|Default|GetACWR_MAG) true)))))

(event Input|MouseEvents|LeftMouseButton
  (params (Key :type Key%20Structure))
  (bind _returnvalue (Game|GetPlayerCharacter 0))
  (bind _astop_down_character (Utilities|Casting|CastToTopDownCharacter _returnvalue))
  (:Pressed
    (Math|Integer|CompareInt (Variables|/Game/TopDownBP/Blueprints/TopDownCharacter.TopDownCharacter_C|GetBulletcount _astop_down_character)
      (:==
        _)
      (:<
        _))
    (bind _output_get (Variables|/Game/TopDownBP/Blueprints/TopDownCharacter.TopDownCharacter_C|SetEmpty? _astop_down_character true))
    (if _output_get
      _)))

(fn ConstructionScript)