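; First-person gun actor that fires pistol bullets when the TopDownCharacter switches to first-person view.
; Entering that mode turns off the gun meshes' shadows and enables shooting after a delay; leaving restores shadows and resets it.
; Tick polls the held left mouse button, blocks fire while dead or running, and uses a short Delay to throttle shots.
; Each shot spawns a bullet, emitter and sound at the character's FPArrow.
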(event Custom|Activate_FirstPerson
  (Rendering|SetCastShadow (Variables|Default|GetACWR_MAG) false)
  (Utilities|FlowControl|Delay 6.0)
  (Rendering|SetVisibility (Variables|Default|GetAim) false false)
  (Variables|Default|SetActivation_Shooting true)
  (Utilities|FlowControl|Delay 2.0))

(event EventBeginPlay
  (Rendering|SetVisibility (Variables|Default|GetAim) false false))

(event Collision|EventActorBeginOverlap
  (params (OtherActor :type Actor%20Object%20Reference)))

(event EventTick
  (params (DeltaSeconds :type Float%20%28single-precision%29))
  (bind _astop_down_character (Utilities|Casting|CastToTopDownCharacter (Game|GetPlayerCharacter 0)))
  (if (Variables|/Game/TopDownBP/Blueprints/TopDownCharacter.TopDownCharacter_C|GetCharacter_Is_Death _astop_down_character)
    (Rendering|SetVisibility (Variables|Default|GetAim) false false)
    (elif (Variables|/Game/TopDownBP/Blueprints/TopDownCharacter.TopDownCharacter_C|GetSwitch_To_First_Person _astop_down_character)
      (Utilities|FlowControl|Sequence
        (:then_0
          (Utilities|FlowControl|DoOnce false :!label _label
            (:Completed
              (CallFunction|ActivateFirstPerson))))
        (:then_1
          (if (Math|Boolean|ANDBoolean (Game|Player|IsInputKeyDown (Game|GetPlayerController 0) "LeftMouseButton") (Variables|Default|GetActivation_Shooting) (not (Variables|/Game/TopDownBP/Blueprints/TopDownCharacter.TopDownCharacter_C|GetCharacter_Is_Death _astop_down_character)) (not (Variables|/Game/TopDownBP/Blueprints/TopDownCharacter.TopDownCharacter_C|GetCharacter_Running _astop_down_character)))
            (Utilities|FlowControl|Delay 0.1)
            (Game|SpawnActorfromClass "/Game/TopDownBP/Blueprints/Weapons/PistolBullet.PistolBullet_C" (Transformation|GetWorldTransform (Variables|/Game/TopDownBP/Blueprints/TopDownCharacter.TopDownCharacter_C|GetFP_Arrow _astop_down_character)) "Undefined" 0 0)
            (Effects|SpawnEmitteratLocation 0 (Transformation|GetWorldLocation (Variables|/Game/TopDownBP/Blueprints/TopDownCharacter.TopDownCharacter_C|GetFP_Arrow _astop_down_character)) "0, 0, 0" "0.050000,0.050000,0.050000")
            (Audio|SpawnSoundatLocation "/Game/FPWeapon/Single_Shot_Cue.Single_Shot_Cue" (Transformation|GetWorldLocation (Variables|/Game/TopDownBP/Blueprints/TopDownCharacter.TopDownCharacter_C|GetFP_Arrow _astop_down_character)) "0, 0, 0" 1.0 1.0 0.0 0 0))))
      (else
        (Rendering|SetVisibility (Variables|Default|GetAim) false false)
        (Rendering|SetCastShadow (Variables|Default|GetACWR_MAG) true)
        (Variables|Default|SetActivation_Shooting false)
        (goto _label Reset)))))

(fn ConstructionScript)