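; Cold storage room Blueprint that switches each of its four walls over to a door variant when that wall's trigger component is overlapped.
; Each Wall M component's begin-overlap event activates the matching Wall Door component and deactivates itself through SetActive, with no filter on the overlapping actor.
; No logic reverses the switch, and the construction script is empty.
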(event OnComponentBeginOverlap(Wall4M)
  (params (OverlappedComponent :type Primitive%20Component%20Object%20Reference) (OtherActor :type Actor%20Object%20Reference) (OtherComp :type Primitive%20Component%20Object%20Reference) (OtherBodyIndex :type Integer) (bFromSweep :type Boolean) (SweepResult :type Hit%20Result%20Structure%20%28by%20ref%29))
  ;[1 1 1] Wall4 Door Switch
  (Components|Activation|SetActive (Variables|Default|GetWall4Door) true false)
  (Components|Activation|SetActive (Variables|Default|GetWall4M) false false))

(event OnComponentBeginOverlap(Wall1M)
  (params (OverlappedComponent :type Primitive%20Component%20Object%20Reference) (OtherActor :type Actor%20Object%20Reference) (OtherComp :type Primitive%20Component%20Object%20Reference) (OtherBodyIndex :type Integer) (bFromSweep :type Boolean) (SweepResult :type Hit%20Result%20Structure%20%28by%20ref%29))
  ;[1 1 1] Wall 1 Door Switch
  (Components|Activation|SetActive (Variables|Default|GetWall1Door) true false)
  (Components|Activation|SetActive (Variables|Default|GetWall1M) false false))

(event OnComponentBeginOverlap(Wall2M)
  (params (OverlappedComponent :type Primitive%20Component%20Object%20Reference) (OtherActor :type Actor%20Object%20Reference) (OtherComp :type Primitive%20Component%20Object%20Reference) (OtherBodyIndex :type Integer) (bFromSweep :type Boolean) (SweepResult :type Hit%20Result%20Structure%20%28by%20ref%29))
  ;[1 1 1] Wall 2 Door Switch
  (Components|Activation|SetActive (Variables|Default|GetWall2Door) true false)
  (Components|Activation|SetActive (Variables|Default|GetWall2M) false false))

(event OnComponentBeginOverlap(Wall3M)
  (params (OverlappedComponent :type Primitive%20Component%20Object%20Reference) (OtherActor :type Actor%20Object%20Reference) (OtherComp :type Primitive%20Component%20Object%20Reference) (OtherBodyIndex :type Integer) (bFromSweep :type Boolean) (SweepResult :type Hit%20Result%20Structure%20%28by%20ref%29))
  ;[1 1 1] Wall 3 Door Switch
  (Components|Activation|SetActive (Variables|Default|GetWall3Door) true false)
  (Components|Activation|SetActive (Variables|Default|GetWall3M) false false))

(event EventBeginPlay)

(event Collision|EventActorBeginOverlap
  (params (OtherActor :type Actor%20Object%20Reference)))

(event EventTick
  (params (DeltaSeconds :type Float%20%28single-precision%29)))

(fn ConstructionScript)